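; BP_AnotherEnemy is a melee enemy that chases the third-person player, damages them and awards score on death.
; Pawn sensing latches CanSeePlayer and triggers an AI MoveTo, which on arrival subtracts Health unless the player's invincibility frames are active.
; Tick counts down the attack cooldown per frame rather than by delta time, and stops movement after a delay while no player has been seen.
; Die adds PointVal to the player's score before destroying the actor.
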(event OnSeePawn(PawnSensing)
  (params (Pawn :type Pawn%20Object%20Reference))
  (Variables|Default|SetCanSeePlayer true)
  (CallFunction|FollowPlayer))

(event Custom|Die
  (bind _returnvalue (Actor|GetActorOfClass "/Game/ThirdPerson/Blueprints/BP_ThirdPersonCharacter.BP_ThirdPersonCharacter_C"))
  (Variables|/Game/ThirdPerson/Blueprints/BP_ThirdPersonCharacter.BP_ThirdPersonCharacter_C|SetScoreAdd _returnvalue (+ (Variables|/Game/ThirdPerson/Blueprints/BP_ThirdPersonCharacter.BP_ThirdPersonCharacter_C|GetScoreAdd _returnvalue) (Variables|Default|GetPointVal)))
  (Actor|DestroyActor))

(event Custom|FollowPlayer
  (if (and (Variables|Default|GetCanSeePlayer) (Variables|Default|GetCanAttack))
    (bind _returnvalue (Actor|GetActorOfClass "/Game/ThirdPerson/Blueprints/BP_ThirdPersonCharacter.BP_ThirdPersonCharacter_C"))
    (AI|AIMoveTo self "0, 0, 0" _returnvalue 7e+01 false
      (:OnSuccess
        (if (Variables|Default|GetCanAttack)
          (Variables|Default|SetCanAttack false)
          (if (<= (Variables|/Game/ThirdPerson/Blueprints/BP_ThirdPersonCharacter.BP_ThirdPersonCharacter_C|GetIFrames _returnvalue) 0.0)
            (Variables|/Game/ThirdPerson/Blueprints/BP_ThirdPersonCharacter.BP_ThirdPersonCharacter_C|SetHealth _returnvalue (- (Variables|/Game/ThirdPerson/Blueprints/BP_ThirdPersonCharacter.BP_ThirdPersonCharacter_C|GetHealth _returnvalue) (Variables|Default|GetDamage)))
            (Variables|/Game/ThirdPerson/Blueprints/BP_ThirdPersonCharacter.BP_ThirdPersonCharacter_C|SetIFrames _returnvalue 3e+01)))))))

(event EventBeginPlay)

(event Collision|EventActorBeginOverlap
  (params (OtherActor :type Actor%20Object%20Reference)))

(event EventTick
  (params (DeltaSeconds :type Float%20%28single-precision%29))
  (Utilities|FlowControl|Sequence
    (:then_0
      (if (not (Variables|Default|GetCanAttack))
        (Variables|Default|SetAttackCooldown (- (Variables|Default|GetAttackCooldown) 1.0))
        (if (<= (Variables|Default|GetAttackCooldown) 0.0)
          (Variables|Default|SetCanAttack true)
          (Variables|Default|SetAttackCooldown 6e+01))))
    (:then_1
      (if (not (Variables|Default|GetCanSeePlayer))
        (Utilities|FlowControl|Delay 2.0)
        (Components|Movement|StopMovementImmediately (Variables|Character|GetCharacterMovement))))))

(fn ConstructionScript)