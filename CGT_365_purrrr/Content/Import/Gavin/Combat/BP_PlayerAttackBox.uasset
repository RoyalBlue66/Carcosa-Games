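; Short-lived player attack hitbox actor that damages BP_AnotherEnemy on overlap, then destroys itself.
; A hit subtracts Damage, optionally launches the enemy up and diagonally away from the player using per-axis signs and ForceMultiplier, and calls Die at zero health.
; The score timer and combo update casts the overlapped enemy, not the player, to BP_ThirdPersonCharacter.
; Lifetime counts down per tick, so duration depends on frame rate.
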(event EventBeginPlay)

(event Collision|EventActorBeginOverlap
  (params (OtherActor :type Actor%20Object%20Reference))
  (bind _forcemultiplier (Variables|Default|GetForceMultiplier))
  (if (Class|GameplayStatics|ObjectIsA OtherActor "/Game/Import/Gavin/Combat/BP_AnotherEnemy.BP_AnotherEnemy_C")
    (Utilities|FlowControl|Sequence
      (:then_0
        (bind _asbp_third_person_character (Utilities|Casting|CastToBP_ThirdPersonCharacter OtherActor))
        (Variables|/Game/ThirdPerson/Blueprints/BP_ThirdPersonCharacter.BP_ThirdPersonCharacter_C|SetScoreTimer _asbp_third_person_character 9e+01)
        (Variables|/Game/ThirdPerson/Blueprints/BP_ThirdPersonCharacter.BP_ThirdPersonCharacter_C|SetComboCount _asbp_third_person_character (+ (Variables|/Game/ThirdPerson/Blueprints/BP_ThirdPersonCharacter.BP_ThirdPersonCharacter_C|GetComboCount _asbp_third_person_character) 1.0)))
      (:then_1
        (bind _asbp_another_enemy (Utilities|Casting|CastToBP_AnotherEnemy OtherActor))
        (Variables|/Game/Import/Gavin/Combat/BP_AnotherEnemy.BP_AnotherEnemy_C|SetHealth _asbp_another_enemy (- (Variables|/Game/Import/Gavin/Combat/BP_AnotherEnemy.BP_AnotherEnemy_C|GetHealth _asbp_another_enemy) (Variables|Default|GetDamage)))
        (if (Variables|Default|GetCausesForce)
          ;[1 1 1] Get the vector between player and enemy
          (bind _returnvalue (Actor|GetActorOfClass "/Game/ThirdPerson/Blueprints/BP_ThirdPersonCharacter.BP_ThirdPersonCharacter_C"))
          (Character|LaunchCharacter _asbp_another_enemy (Math|Vector|MakeVector (* (/ (- (.X (Math|Vector|BreakVector (Transformation|GetActorLocation _asbp_another_enemy))) (.X (Math|Vector|BreakVector (Transformation|GetActorLocation _returnvalue)))) (Math|Float|Absolute(Float) (- (.X (Math|Vector|BreakVector (Transformation|GetActorLocation _asbp_another_enemy))) (.X (Math|Vector|BreakVector (Transformation|GetActorLocation _returnvalue)))))) _forcemultiplier) (* (/ (- (.Y (Math|Vector|BreakVector (Transformation|GetActorLocation _asbp_another_enemy))) (.Y (Math|Vector|BreakVector (Transformation|GetActorLocation _returnvalue)))) (Math|Float|Absolute(Float) (- (.Y (Math|Vector|BreakVector (Transformation|GetActorLocation _asbp_another_enemy))) (.Y (Math|Vector|BreakVector (Transformation|GetActorLocation _returnvalue)))))) _forcemultiplier) _forcemultiplier) true true))
        (if (<= (Variables|/Game/Import/Gavin/Combat/BP_AnotherEnemy.BP_AnotherEnemy_C|GetHealth _asbp_another_enemy) 0.0)
          (Default|Die _asbp_another_enemy))
        (Actor|DestroyActor)))))

(event EventTick
  (params (DeltaSeconds :type Float%20%28single-precision%29))
  (Variables|Default|SetLifetime (- (Variables|Default|GetLifetime) 1.0))
  (if (<= (Variables|Default|GetLifetime) 0.0)
    (Actor|DestroyActor)))

(fn ConstructionScript)