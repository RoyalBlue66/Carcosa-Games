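; Player weapon actor configured by a WeaponInfo struct that sets its mesh, attack VFX, sound, damage and knockback.
; SpawnVFX spawns the Niagara effect attached to the weapon or aimed at the cursor location, passes itself in as PlayerWeapon and plays the sound.
; Particles drive hit detection: ParticleData sphere-traces at each exported particle, damages the nearest enemy and optionally launches it backward.
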(event Custom|SpawnVFX
  (params (CursorLoc :type Vector))
  (bind _returnvalue (Components|GetOwner))
  (bind _self self)
  (bind _weapon (Variables|Default|GetWeapon))
  (bind _weaponinfo (Variables|Default|GetWeaponInfo))
  (bind _weaponinfo_2 (Variables|Default|GetWeaponInfo))
  (bind (_attacksound _vfx _attachtoweapon) (Utilities|Struct|BreakS_Player_WeaponInfo _weaponinfo))
  (bind _fxfromweapon (Utilities|Struct|BreakS_Player_WeaponInfo _weaponinfo_2))
  (bind _returnvalue_2 (Transformation|GetSocketLocation _weapon "FX_Handle"))
  (bind _asbp_third_person_character (Utilities|Casting|CastToBP_ThirdPersonCharacter _returnvalue))
  (bind _mesh (Variables|/Script/Engine.Character|GetMesh _asbp_third_person_character))
  (bind _returnvalue_3 (Transformation|GetWorldLocation _mesh))
  (bind _returnvalue_4 (+ _returnvalue_3 "0.000000,0.000000,10.000000"))
  (bind _returnvalue_5 (Math|Vector|SelectVector _returnvalue_2 _returnvalue_4 _fxfromweapon))
  (bind _returnvalue_6 (Math|Rotator|FindLookatRotation _returnvalue_5 CursorLoc))
  (if _attachtoweapon
    (bind _returnvalue_7 (Niagara|SpawnSystemAttached _vfx (Variables|Default|GetWeapon) "FX_Handle" "0, 0, 0" (Math|Rotator|MakeRotator 0.0 0.0 0.0) "KeepRelativeOffset" true))
    (Niagara|SetNiagaraVariable(Object) _returnvalue_7 "PlayerWeapon" _self)
    (else
      (bind _returnvalue_8 (Niagara|SpawnSystematLocation _vfx _returnvalue_5 (Math|Rotator|MakeRotator (.roll _returnvalue_6) 0.0 (.yaw _returnvalue_6))))
      (Niagara|SetNiagaraVariable(Object) _returnvalue_8 "PlayerWeapon" _self)))
  (Audio|SpawnSound2D _attacksound 1.0 1.0 0.0 0))

(event EventBeginPlay)

(event Collision|EventActorBeginOverlap
  (params (OtherActor :type Actor%20Object%20Reference)))

(event EventTick
  (params (DeltaSeconds :type Float%20%28single-precision%29)))

(event EventParticleData
  (params (Data :type Array%20of%20Basic%20Particle%20Data%20Structures) (NiagaraSystem :type Niagara%20System%20Object%20Reference) (SimulationPositionOffset :type Vector%20%28by%20ref%29 :default "0, 0, 0"))
  (bind _weaponinfo (Variables|Default|GetWeaponInfo))
  (bind (_damage _applyforce) (Utilities|Struct|BreakS_Player_WeaponInfo _weaponinfo))
  (for _array_element Data
    (bind _outhits (Collision|MultiSphereTraceForObjects (.Position (Utilities|Struct|BreakBasicParticleData _array_element)) (+ (.Position (Utilities|Struct|BreakBasicParticleData _array_element)) "0.000000,0.000000,50.000000") (.Size (Utilities|Struct|BreakBasicParticleData _array_element)) (Utilities|Array|MakeArray "ObjectTypeQuery9") false 0 "ForDuration" true "(R=1.000000,G=0.000000,B=0.000000,A=1.000000)" "(R=0.000000,G=1.000000,B=0.000000,A=1.000000)" 1.0))
    (for _array_element_2 _outhits
      (Utilities|Array|Add (Variables|Default|GetTempVar) (.HitActor (Collision|BreakHitResult _array_element_2))))
    (bind _asbp_enemy_base (Utilities|Casting|CastToBP_EnemyBase (.ReturnValue (Actor|FindNearestActor (.Position (Utilities|Struct|BreakBasicParticleData _array_element)) (Variables|Default|GetTempVar)))))
    (Game|Damage|ApplyDamage (.ReturnValue (Actor|FindNearestActor (.Position (Utilities|Struct|BreakBasicParticleData _array_element)) (Variables|Default|GetTempVar))) _damage 0 0)
    (if (and _applyforce (Utilities|Enum|NotEqual(Enum) (Variables|/Script/Engine.CharacterMovementComponent|GetMovementMode (Variables|/Script/Engine.Character|GetCharacterMovement _asbp_enemy_base)) "MOVE_Falling"))
      (Default|Launch _asbp_enemy_base (* (+ (Math|Vector|NegateVector (Transformation|GetActorForwardVector _asbp_enemy_base)) "0.000000,0.000000,0.600000") 7.5e+02 (+ (Math|Float|Max(Float) (- 1.0 (.X (Math|Vector|BreakVector (.Velocity (Utilities|Struct|BreakBasicParticleData _array_element))))) 0.5) 0.3))))
    (Variables|Default|SetTempVar (Utilities|Array|MakeArray 0))))

(fn ConstructionScript)

(fn SetWeapon
  (params (WeaponInfo :type S%20Player%20Weapon%20Info%20Structure))
  (bind _output_get (Variables|Default|SetWeaponInfo WeaponInfo))
  (Components|StaticMesh|SetStaticMesh (Variables|Default|GetWeapon) (.Mesh (Utilities|Struct|BreakS_Player_WeaponInfo _output_get))))