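; BP_PlayerAttackProjectile is a player attack projectile that travels in a straight line along its local forward axis.
; BeginPlay sets Lifetime before calling the parent, and nothing in this graph reads that value.
; Each Tick moves the root component forward by a fixed, swept step that is not scaled by DeltaSeconds, so speed depends on frame rate.
; The overlap event is disabled, so this graph has no hit logic.
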(event EventBeginPlay
  (Variables|Default|SetLifetime 6e+02)
  (|CallParentFunction))

(event Collision|EventActorBeginOverlap
  (params (OtherActor :type Actor%20Object%20Reference))
  (|CallParentFunction OtherActor) ; This node is disabled and will not be called.\nDrag off pins to build functionality.
)

(event EventTick
  (params (DeltaSeconds :type Float%20%28single-precision%29))
  (Class|SceneComponent|AddLocalTransform (Variables|Default|GetDefaultSceneRoot) (Math|Transform|MakeTransform "24.000000,0.000000,0.000000") true false)
  (|CallParentFunction DeltaSeconds))

(fn ConstructionScript
  (|CallParentFunction))