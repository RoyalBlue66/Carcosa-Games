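; BP_WinterBranchDummy is a player character test Blueprint with score, damage and slow-down debuff logic.
; Incoming damage subtracts from Score as a stand-in for health and prints a message, while AddScore increases it.
; SlowDown lowers walk speed and records the time; a looping timer calls SpeedUp, restoring speed once enough time has passed since the latest hit of the debuff.
; The DebuffStacks RepNotify only prints a constant.
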(event Custom|SpeedUp
  ;[1 1 1] Slow Down Debuff, SpeedUp Function Allows Timer Reset
  (if (>= (- (Utilities|Time|GetGameTimeinSeconds) (Variables|Default|GetSlowTimer)) 2.0)
    (Variables|/Script/Engine.CharacterMovementComponent|SetMaxWalkSpeed (Variables|Character|GetCharacterMovement) 7.5e+02)))

(event Custom|AddScore
  (params (Score :type Float%20%28double-precision%29))
  (Variables|Default|SetScore (+ (Variables|Default|GetScore) Score)))

(event Custom|SlowDown
  ;[1 1 1] Slow Down Debuff, SpeedUp Function Allows Timer Reset
  (Variables|Default|SetSlowTimer (Utilities|Time|GetGameTimeinSeconds))
  (Variables|/Script/Engine.CharacterMovementComponent|SetMaxWalkSpeed (Variables|Character|GetCharacterMovement) 6e+02)
  (Utilities|Time|SetTimerbyEvent (delegate Custom|SpeedUp) 1.0 true))

(event Game|Damage|EventAnyDamage
  (params (Damage :type Float%20%28single-precision%29) (DamageType :type Damage%20Type%20Object%20Reference) (InstigatedBy :type Controller%20Object%20Reference) (DamageCauser :type Actor%20Object%20Reference))
  ;[1 1 1] Player takes damage, i did see a health variable, so damage -= score, for now, Benny
  (Variables|Default|SetScore (- (Variables|Default|GetScore) Damage))
  (Development|PrintString "Ouch"))

(fn ConstructionScript)

(fn OnRepDebuffStacks
  (Development|PrintString (Utilities|String|ToString(Integer) 0)))