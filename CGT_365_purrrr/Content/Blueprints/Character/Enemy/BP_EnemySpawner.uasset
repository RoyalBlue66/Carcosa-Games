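; Enemy spawner that periodically spawns a random enemy type from DT_EnemyStats at its Indicator while AllowSpawn is on.
; BeginPlay and the AllowSpawn RepNotify control looping timers that spin the Indicator and run SelectEnemyType.
; SelectEnemyType makes a weighted pick by subtracting each row's SpawnRate from a random roll.
; Multi-spawn types appear as random-sized groups scattered within SpawnRadius, others singly, each given its default controller.
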(event Custom|StartSpawn
  (Utilities|Time|SetTimerbyFunctionName 0 "IndicatorSpin" 0.1 true)
  (Utilities|Time|SetTimerbyFunctionName 0 "SelectEnemyType" 3.0 true))

(event Custom|StopSpawn
  (Utilities|Time|ClearTimerbyFunctionName 0 "SelectEnemyType")
  (Utilities|Time|ClearTimerbyFunctionName 0 "IndicatorSpin"))

(event EventBeginPlay
  (Utilities|FlowControl|Sequence
    (:then_0
      (Rendering|SetVisibility (Variables|Default|GetIndicator) (Variables|Default|GetVisiableIndicator) false))
    (:then_1
      (bind _outrownames (DataTable|GetDataTableRowNames "/Game/Blueprints/Data/EnemyStats/DT_EnemyStats.DT_EnemyStats"))
      (Variables|Default|SetEnemyTypes _outrownames))
    (:then_2
      (if (Variables|Default|GetAllowSpawn)
        (CallFunction|StartSpawn)))))

(fn ConstructionScript)

(fn IndicatorSpin
  (Transformation|AddRelativeRotation (Variables|Default|GetIndicator) "0.000000,20.000000,0.000000" false false))

(fn EnemySpawnSinglePt
  (params (EnemyData :type Actor%20Class%20Reference))
  (bind _indicator (Variables|Default|GetIndicator))
  (bind _returnvalue (Transformation|GetWorldTransform _indicator))
  (bind _returnvalue_2 (Game|SpawnActorfromClass EnemyData (Math|Transform|MakeTransform (.location _returnvalue) (.rotation _returnvalue) "1.000000,1.000000,1.000000") "AdjustIfPossibleButAlwaysSpawn" "MultiplyWithRoot" self 0))
  (bind _asbp_enemy_base (Utilities|Casting|CastToBP_EnemyBase _returnvalue_2))
  (Pawn|SpawnDefaultController _asbp_enemy_base))

(fn EnemySpawnRange
  (params (Enemy :type Actor%20Class%20Reference))
  (bind _indicator (Variables|Default|GetIndicator))
  (bind _spawnradius (Variables|Default|GetSpawnRadius))
  (bind _returnvalue (Transformation|GetWorldTransform _indicator))
  (bind _returnvalue_2 (* _spawnradius -1.0))
  (bind _returnvalue_3 (Math|Random|RandomFloatinRange _returnvalue_2 _spawnradius))
  (bind _returnvalue_4 (Game|SpawnActorfromClass Enemy (Math|Transform|MakeTransform (Math|Vector|MakeVector (+ (.x (.location _returnvalue)) _returnvalue_3) (+ (.y (.location _returnvalue)) _returnvalue_3) (.z (.location _returnvalue))) (.rotation _returnvalue) "1.000000,1.000000,1.000000") "AdjustIfPossibleButAlwaysSpawn" "MultiplyWithRoot" self 0))
  (bind _asbp_enemy_base (Utilities|Casting|CastToBP_EnemyBase _returnvalue_4))
  (Pawn|SpawnDefaultController _asbp_enemy_base))

(fn OnRepAllowSpawn
  (if (Variables|Default|GetAllowSpawn)
    (CallFunction|StartSpawn)
    (else
      (CallFunction|StopSpawn))))

(fn SelectEnemyType
  (LocalVariables|SetSpawnCheck (Math|Random|RandomFloat))
  (bind _array_element (Utilities|Array|ForEachLoopwithBreak (Variables|Default|GetEnemyTypes) :!label _label)
    (:LoopBody
      (bind _returnvalue (Utilities|GetDataTableRow "/Game/Blueprints/Data/EnemyStats/DT_EnemyStats.DT_EnemyStats" _array_element)
        (:then
          (if (>= (.SpawnRate (Utilities|Struct|BreakS_EnemyStats _returnvalue)) (LocalVariables|GetSpawnCheck))
            (LocalVariables|SetChosenEnemy _returnvalue)
            (goto _label Break)
            (else
              (|SetBy-RefVar (LocalVariables|GetSpawnCheck) (- (LocalVariables|GetSpawnCheck) (.SpawnRate (Utilities|Struct|BreakS_EnemyStats _returnvalue)))))))))
    (:Completed
      (if (.SpawnMulti (Utilities|Struct|BreakS_EnemyStats (LocalVariables|GetChosenEnemy)))
        (for _index (range 1 (Math|Random|RandomIntegerinRange (.SpawnMultiMin (Utilities|Struct|BreakS_EnemyStats (LocalVariables|GetChosenEnemy))) (.SpawnMultiMax (Utilities|Struct|BreakS_EnemyStats (LocalVariables|GetChosenEnemy)))))
          (CallFunction|EnemySpawnRange (.BP (Utilities|Struct|BreakS_EnemyStats (LocalVariables|GetChosenEnemy)))))
        (else
          (CallFunction|EnemySpawnSinglePt (.BP (Utilities|Struct|BreakS_EnemyStats (LocalVariables|GetChosenEnemy)))))))))