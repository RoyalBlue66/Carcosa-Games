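; Fluffball enemy Blueprint that attacks the player with an exploding radial-damage burst and Niagara effect.
; Tick and landing check for the player within attack range while falling, then set Attacking and disable Tick.
; Otherwise, landing focuses the AI controller on the player and restarts its two-second move timer.
; Launch ignores Pawn collision, calls LaunchCharacter and pauses that timer.
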(event Custom|Attack%20Player
  (bind _returnvalue (Transformation|GetActorLocation))
  (bind _enemystats (Variables|Default|GetEnemyStats))
  (bind (_attackdamage _attackrange) (Utilities|Struct|BreakS_EnemyStats _enemystats))
  ;[1 1 1] Prepare and then Explode. Adjust Delay if necessary.
  (Niagara|SpawnSystematLocation "/Game/Assets/VFX/Enemy/NS_Fluffball_Explode.NS_Fluffball_Explode" (- _returnvalue "0.000000,0.000000,48.000000"))
  (Game|Damage|ApplyRadialDamage _attackdamage _returnvalue _attackrange 0 0 0 0 true "ECC_GameTraceChannel2"))

(event EventOnLanded
  (params (Hit :type Hit%20Result%20Structure%20%28by%20ref%29))
  (bind _aic (Variables|Default|GetAIC))
  (bind _asaic_fluffball (Utilities|Casting|CastToAIC_Fluffball _aic))
  (Variables|Default|SetMoving false)
  (Utilities|Time|ClearandInvalidateTimerbyHandle (Variables|/Game/Blueprints/Character/Enemy/Controllers/AIC_Fluffball.AIC_Fluffball_C|GetMoveTimer _asaic_fluffball))
  (CallFunction|CheckAttackDistance)
  (if (not (Variables|Default|GetAttacking))
    (AI|SetFocus _asaic_fluffball (Variables|/Game/Blueprints/Character/Enemy/Controllers/AIC_Fluffball.AIC_Fluffball_C|GetPlayerCharacter _asaic_fluffball))
    (bind _returnvalue (Utilities|Time|SetTimerbyEvent (EventDispatchers|CreateEvent _asaic_fluffball :!event MovetoPlayer) 2.0))
    (Variables|/Game/Blueprints/Character/Enemy/Controllers/AIC_Fluffball.AIC_Fluffball_C|SetMoveTimer _asaic_fluffball _returnvalue)))

(event EventTick
  (params (DeltaSeconds :type Float%20%28single-precision%29))
  (CallFunction|CheckAttackDistance))

(event EventLaunch
  (params (Velocity :type Vector :default "0, 0, 0"))
  (bind _aic (Variables|Default|GetAIC))
  (bind _asaic_fluffball (Utilities|Casting|CastToAIC_Fluffball _aic))
  (bind _movetimer (Variables|/Game/Blueprints/Character/Enemy/Controllers/AIC_Fluffball.AIC_Fluffball_C|GetMoveTimer _asaic_fluffball))
  (Collision|SetCollisionResponsetoChannel (Variables|Default|GetCapsuleComponent) "ECC_Pawn" "ECR_Ignore")
  (Character|LaunchCharacter "0, 0, 0" true true)
  (if (Utilities|Time|IsValidTimerHandle _movetimer)
    (Utilities|Time|PauseTimerbyHandle _movetimer)))

(event EventTryAttack)

(event EventBeginPlay
  (|CallParentFunction))

(fn ConstructionScript)

(fn CheckAttackDistance
  (if (not (or (> (Transformation|GetDistanceTo (Game|GetPlayerCharacter 0)) (.AttackRange (Utilities|Struct|BreakS_EnemyStats (Variables|Default|GetEnemyStats)))) (Utilities|Enum|NotEqual(Enum) (Variables|/Script/Engine.CharacterMovementComponent|GetMovementMode (Variables|Character|GetCharacterMovement)) "MOVE_Falling")))
    (Variables|Default|SetAttacking true)
    (Actor|Tick|SetActorTickEnabled false)))