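; BP_EnemyGhastly is an enemy character variant that sets its own default stats before running the parent BeginPlay.
; Its TryAttack applies CurrentDamage directly to the player character, with no range check in this graph.
; A CanAttack flag and a one-shot timer of TimeBetweenAttacks act as the cooldown between hits.
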(event Custom|ResetAttack
  (Variables|Default|SetbCanAttack true))

(event EventTryAttack
  (if (Variables|Default|GetbCanAttack)
    (Variables|Default|SetbCanAttack false)
    (bind _asbp_third_person_character (Utilities|Casting|CastToBP_ThirdPersonCharacter (Game|GetPlayerCharacter 0)))
    (Game|Damage|ApplyDamage _asbp_third_person_character (Variables|Default|GetCurrentDamage) 0 0)
    (Utilities|Time|SetTimerbyEvent (delegate Custom|ResetAttack) (Variables|Default|GetTimeBetweenAttacks))))

(event EventBeginPlay
  (Variables|Default|SetDefaultStats (Utilities|Struct|MakeS_EnemyStats 2e+02 4e+02 2e+01 3.6e+02 0.5 1e+02 1.5))
  (|CallParentFunction))

(fn ConstructionScript)