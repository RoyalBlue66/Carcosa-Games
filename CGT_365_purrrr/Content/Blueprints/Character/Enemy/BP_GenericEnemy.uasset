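; Generic enemy actor that turns toward the third-person player every tick and steps forward, without sweep, while Walk is true.
; Shovebox overlaps with other enemies jump it by random X/Y offsets to separate them.
; Hurtbox overlaps halt walking and subtract health directly from the player's HUD health bar, with delays gating the next hit and movement.
; Die adds the enemy's point value to the player's score and destroys it.
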(event OnComponentBeginOverlap(Shovebox)
  (params (OverlappedComponent :type Primitive%20Component%20Object%20Reference) (OtherActor :type Actor%20Object%20Reference) (OtherComp :type Primitive%20Component%20Object%20Reference) (OtherBodyIndex :type Integer) (bFromSweep :type Boolean) (SweepResult :type Hit%20Result%20Structure%20%28by%20ref%29))
  (bind _returnvalue (Transformation|GetActorLocation))
  (Utilities|Casting|CastToBP_GenericEnemy OtherActor)
  (Variables|Default|SetWalk false)
  (bind _float (CallFunction|RandomDistance))
  (bind _float_2 (CallFunction|RandomDistance))
  (Transformation|SetActorRelativeLocation (Math|Vector|MakeVector (+ _float (.x _returnvalue)) (+ _float_2 (.y _returnvalue)) (.z _returnvalue)))
  (Variables|Default|SetWalk true))

(event OnComponentBeginOverlap(Hurtbox)
  (params (OverlappedComponent :type Primitive%20Component%20Object%20Reference) (OtherActor :type Actor%20Object%20Reference) (OtherComp :type Primitive%20Component%20Object%20Reference) (OtherBodyIndex :type Integer) (bFromSweep :type Boolean) (SweepResult :type Hit%20Result%20Structure%20%28by%20ref%29))
  ;[1 1 1] Stop Moving and Attack Player
  (Variables|Default|SetWalk false)
  (bind _asbp_third_person_character (Utilities|Casting|CastToBP_ThirdPersonCharacter OtherActor))
  (Variables|/Game/Blueprints/UI/GUI_HUD/HUD_HealthBars.HUD_HealthBars_C|SetCurrentHealth (Variables|/Game/Blueprints/UI/GUI_HUD/HUD_Container.HUD_Container_C|GetHUD_HealthBars (Variables|/Game/Blueprints/Character/Player/BP_ThirdPersonCharacter.BP_ThirdPersonCharacter_C|GetHUD%20Container _asbp_third_person_character)) (- (Variables|/Game/Blueprints/UI/GUI_HUD/HUD_HealthBars.HUD_HealthBars_C|GetCurrentHealth (Variables|/Game/Blueprints/UI/GUI_HUD/HUD_Container.HUD_Container_C|GetHUD_HealthBars (Variables|/Game/Blueprints/Character/Player/BP_ThirdPersonCharacter.BP_ThirdPersonCharacter_C|GetHUD%20Container _asbp_third_person_character))) 5))
  (Development|PrintString "OUCH!!!")
  (Collision|SetCollisionEnabled (Variables|Default|GetHurtbox) "NoCollision")
  (Utilities|FlowControl|Delay 1.0)
  (Collision|SetCollisionEnabled (Variables|Default|GetHurtbox) "QueryOnly")
  (Variables|Default|SetWalk true))

(event OnComponentEndOverlap(Hurtbox)
  (params (OverlappedComponent :type Primitive%20Component%20Object%20Reference) (OtherActor :type Actor%20Object%20Reference) (OtherComp :type Primitive%20Component%20Object%20Reference) (OtherBodyIndex :type Integer))
  ;[1 1 1] Stop Moving and Attack Player
  (Utilities|FlowControl|Delay 0.5)
  (Variables|Default|SetWalk true))

(event Custom|Die
  (bind _returnvalue (Actor|GetActorOfClass "/Game/Blueprints/Character/Player/BP_ThirdPersonCharacter.BP_ThirdPersonCharacter_C"))
  (Variables|/Game/Blueprints/Character/Player/BP_ThirdPersonCharacter.BP_ThirdPersonCharacter_C|SetScoreAdd _returnvalue (+ (Variables|/Game/Blueprints/Character/Player/BP_ThirdPersonCharacter.BP_ThirdPersonCharacter_C|GetScoreAdd _returnvalue) (Variables|Default|GetPointVal)))
  (Actor|DestroyActor))

(event EventTick
  (params (DeltaSeconds :type Float%20%28single-precision%29))
  (bind _returnvalue (Transformation|GetActorForwardVector))
  (bind _returnvalue_2 (* _returnvalue 6.0))
  ;[1 1 1] Look At And Approach Player
  (bind _returnvalue_3 (Actor|GetActorOfClass "/Game/Blueprints/Character/Player/BP_ThirdPersonCharacter.BP_ThirdPersonCharacter_C"))
  (Transformation|SetActorRotation (Math|Rotator|MakeRotator 0.0 0.0 (.yaw (Math|Rotator|FindLookatRotation (Transformation|GetActorLocation) (Transformation|GetActorLocation _returnvalue_3)))))
  (if (Variables|Default|GetWalk)
    (Transformation|SetActorRelativeLocation (+ (Transformation|GetActorLocation) (Math|Vector|MakeVector (.x _returnvalue_2) (.y _returnvalue_2) 0.0)))))

(fn ConstructionScript)

(fn RandomDistance
  (bind _returnvalue (Math|Random|RandomFloatinRange 1e+01 5e+01))
  ;[1 1 1] Create A Random Distance of -50 to -10 or 10 to 50
  (if (== (Math|Random|RandomIntegerinRange 1 2) 1)
    (bind _result (Math|Float|NegateFloat _returnvalue)
      (:%20%20
        (return _result)))
    (else
      (return _returnvalue))))