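; BP_EnemyHisswalker is an enemy character that periodically bursts into a sprint and damages the player.
; BeginPlay sets its DefaultStats before running the parent BeginPlay, then starts a looping timer that briefly boosts walk speed every few seconds before restoring DefaultSpeed.
; TryAttack applies CurrentDamage directly to the player character, with no range check here, and uses a timer-reset CanAttack flag as cooldown.
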(event Custom|SpeedUp
  ;[1 1 1] Speed Up Every 5 Seconds For 1 Second
  (Variables|/Script/Engine.CharacterMovementComponent|SetMaxWalkSpeed (Variables|Character|GetCharacterMovement) 1e+03)
  (Utilities|FlowControl|Delay 1.0)
  (Variables|/Script/Engine.CharacterMovementComponent|SetMaxWalkSpeed (Variables|Character|GetCharacterMovement) (Variables|Default|GetDefaultSpeed)))

(event Custom|ResetAttack
  ;[1 1 1] Basic Attack Function
  (Variables|Default|SetbCanAttack true))

(event EventTryAttack
  ;[1 1 1] Basic Attack Function
  (if (Variables|Default|GetbCanAttack)
    (Variables|Default|SetbCanAttack false)
    (bind _asbp_third_person_character (Utilities|Casting|CastToBP_ThirdPersonCharacter (Game|GetPlayerCharacter 0)))
    (Game|Damage|ApplyDamage _asbp_third_person_character (Variables|Default|GetCurrentDamage) 0 0)
    (Utilities|Time|SetTimerbyEvent (delegate Custom|ResetAttack) (Variables|Default|GetTimeBetweenAttacks))))

(event EventBeginPlay
  (Variables|Default|SetDefaultStats (Utilities|Struct|MakeS_EnemyStats 1e+02 4e+02 2e+01 1e+02 0.5 1e+02 1.5))
  (|CallParentFunction)
  (Utilities|Time|SetTimerbyEvent (delegate Custom|SpeedUp) 5.0 true))

(fn ConstructionScript)