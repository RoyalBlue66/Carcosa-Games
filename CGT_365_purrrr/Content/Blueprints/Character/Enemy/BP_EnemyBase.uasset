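; Base enemy character that initializes health, speed, damage and attack settings from its DefaultStats struct on BeginPlay.
; OnHit deducts health, then either destroys the actor or launches it away from the player while briefly pausing AIC_DefaultAIC movement.
; Buff events toggle doubled walk speed and halved attack interval, with a short delay if stats are not yet ready.
; TryAttack is a timer-gated placeholder called by the AI controller, meant for child overrides.
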(event Custom|TryAttack
  ;[1 1 1] Base function, OVERRIDE THIS! This is called in AIC_Default
  (if (Variables|Default|GetbCanAttack)
    (Variables|Default|SetbCanAttack false)
    (Development|PrintString "Hey, i just attacked. However, this is a parent function, please override this function in a child blueprint. This should have ~1s cooldown btw.")
    (Utilities|Time|SetTimerbyEvent (delegate Custom|ResetAttactGate) 1.0)))

(event Custom|ResetAttactGate
  ;[1 1 1] Base function, OVERRIDE THIS! This is called in AIC_Default
  (Variables|Default|SetbCanAttack true))

(event Custom|OnHit
  (params (DamageAmount :type Float%20%28double-precision%29) (Projectile :type BP%20Player%20Attack%20Box%20Object%20Reference) (ImpulseStrength :type Float%20%28double-precision%29))
  (bind _returnvalue (Transformation|GetActorLocation))
  (bind _returnvalue_2 (Game|GetPlayerCharacter 0))
  (bind _self self)
  (bind _returnvalue_3 (Transformation|GetActorLocation _returnvalue_2))
  (bind _returnvalue_4 (AI|GetAIController _self))
  (bind _returnvalue_5 (- _returnvalue _returnvalue_3))
  (bind _returnvalue_6 (Class|KismetMathLibrary|VectorNormal2D _returnvalue_5 0.0001))
  ;[1 1 1] Health deduction
  (Variables|RuntimeStats|SetCurrentHealth (Math|Float|Clamp(Float) (- (Variables|RuntimeStats|GetCurrentHealth) DamageAmount) 0.0 (Variables|RuntimeStats|GetMaxHealth)))
  ;[1 1 1] Death check
  (if (<= (Variables|RuntimeStats|GetCurrentHealth) 0.0)
    (CallFunction|OnDeath)
    (else
      ;[1 1 1] Apply knockback
      (bind _asaic_default_aic (Utilities|Casting|CastToAIC_DefaultAIC _returnvalue_4))
      (Variables|/Game/Blueprints/Character/Enemy/AIC_DefaultAIC.AIC_DefaultAIC_C|SetbCanMove _asaic_default_aic false)
      (AI|Navigation|StopMovement _returnvalue_4)
      (Character|LaunchCharacter (* (Math|Vector|MakeVector (.x _returnvalue_6) (.y _returnvalue_6) 0.1) ImpulseStrength) true false)
      (Utilities|FlowControl|Delay 0.5)
      (Variables|/Game/Blueprints/Character/Enemy/AIC_DefaultAIC.AIC_DefaultAIC_C|SetbCanMove _asaic_default_aic true))))

(event Custom|OnDeath
  (Actor|DestroyActor))

(event Custom|BuffActivate
  ;[1 1 1] Buff And Return To Normal Stats, Delay To Ensure Stats are Initialized
  (if (Variables|Default|GetBuffReady)
    _
    (else
      (Utilities|FlowControl|Delay 0.1)))
  (Variables|/Script/Engine.CharacterMovementComponent|SetMaxWalkSpeed (Variables|Character|GetCharacterMovement) (Variables|Default|GetBuffedSpeed))
  (Variables|RuntimeStats|SetTimeBetweenAttacks (Variables|Default|GetBuffedAttackSpeed)))

(event Custom|TEST_PRINTHEALTH
  (Development|PrintString (Utilities|String|ToString(Float) (Variables|RuntimeStats|GetCurrentHealth)) true true "(R=0.000000,G=0.660000,B=1.000000,A=1.000000)" 0.3))

(event Custom|BuffDeactivate
  ;[1 1 1] Buff And Return To Normal Stats, Delay To Ensure Stats are Initialized
  (Variables|/Script/Engine.CharacterMovementComponent|SetMaxWalkSpeed (Variables|Character|GetCharacterMovement) (Variables|RuntimeStats|GetDefaultSpeed))
  (Variables|RuntimeStats|SetTimeBetweenAttacks (Variables|Default|GetDefaultAttackSpeed)))

(event EventBeginPlay
  (bind _defaultstats (Variables|Default|GetDefaultStats))
  (bind (_health _movementspeed _attackdamage _attackrange _attacklandtime _worthscore _timebetweenattack) (Utilities|Struct|BreakS_EnemyStats _defaultstats))
  (Utilities|FlowControl|Sequence
    (:then_0
      ;[1 1 1] Initialize using S_EnemyStats structure, exposed to spawn, Set Buffs
      (bind _output_get (Variables|RuntimeStats|SetCurrentHealth _health))
      (Variables|RuntimeStats|SetMaxHealth _output_get))
    (:then_1
      (bind _output_get_2 (Variables|RuntimeStats|SetCurrentSpeed _movementspeed))
      (bind _output_get_3 (Variables|RuntimeStats|SetDefaultSpeed _output_get_2))
      (bind _output_get_4 (Variables|/Script/Engine.CharacterMovementComponent|SetMaxWalkSpeed (Variables|Character|GetCharacterMovement) _output_get_3))
      (Variables|Default|SetBuffedSpeed (* _output_get_4 2.0)))
    (:then_2
      (bind _output_get_5 (Variables|RuntimeStats|SetCurrentDamage _attackdamage))
      (Variables|RuntimeStats|SetDefaultDamage _output_get_5))
    (:then_3
      (Variables|RuntimeStats|SetAttackRange _attackrange))
    (:then_4
      (Variables|RuntimeStats|SetAttackLandTime _attacklandtime))
    (:then_5
      (Variables|RuntimeStats|SetWorthScore _worthscore))
    (:then_6
      (bind _output_get_6 (Variables|RuntimeStats|SetTimeBetweenAttacks _timebetweenattack))
      (bind _output_get_7 (Variables|Default|SetDefaultAttackSpeed _output_get_6))
      (Variables|Default|SetBuffedAttackSpeed (/ _output_get_7 2.0))
      (Variables|Default|SetBuffReady true))))

(fn ConstructionScript)