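; BP_EnemyFast is a fast enemy character that sets its own default stats on BeginPlay.
; Each tick without an active special, it box-traces toward the player and, on a hit, randomly picks a pounce, leap or speed-boosted hunt.
; Pounce and leap flag the owning AI controller and launch forward; all three share a delayed cooldown.
; Timed attacks swap materials and track an overlapping player, but apply no damage here.
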(event OnComponentBeginOverlap(DamageArea)
  (params (OverlappedComponent :type Primitive%20Component%20Object%20Reference) (OtherActor :type Actor%20Object%20Reference) (OtherComp :type Primitive%20Component%20Object%20Reference) (OtherBodyIndex :type Integer) (bFromSweep :type Boolean) (SweepResult :type Hit%20Result%20Structure%20%28by%20ref%29))
  (bind _asbp_third_person_character (Utilities|Casting|CastToBP_ThirdPersonCharacter OtherActor))
  (Variables|Default|SetAttackTargetRef _asbp_third_person_character))

(event OnComponentEndOverlap(DamageArea)
  (params (OverlappedComponent :type Primitive%20Component%20Object%20Reference) (OtherActor :type Actor%20Object%20Reference) (OtherComp :type Primitive%20Component%20Object%20Reference) (OtherBodyIndex :type Integer))
  (Utilities|Casting|CastToBP_ThirdPersonCharacter OtherActor)
  (Variables|Default|SetAttackTargetRef 0))

(event Custom|OnEndAttack
  (bind _attacktargetref (Variables|Default|GetAttackTargetRef))
  (Rendering|Material|SetMaterial (Variables|Default|GetTEMP_STATIC_EnemyMesh) 0 "/Game/Assets/Materials/Character/Enemy/M_enemy01.M_enemy01")
  (Utilities|IsValid _attacktargetref
    (:Is%20Valid
      (Utilities|Casting|CastToBP_ThirdPersonCharacter _attacktargetref))))

(event Custom|ResetAttackGate
  (Variables|Default|SetbCanAttack true))

(event Custom|Hunting
  (Variables|/Script/Engine.CharacterMovementComponent|SetMaxWalkSpeed (Variables|Character|GetCharacterMovement) 7.5e+02)
  (Variables|Default|SetCurrentSpeed 7.5e+02)
  (Utilities|FlowControl|Delay 6.0)
  (Variables|/Script/Engine.CharacterMovementComponent|SetMaxWalkSpeed (Variables|Character|GetCharacterMovement) 6e+02)
  (Variables|Default|SetCurrentSpeed 6e+02)
  (CallFunction|EndSpecialMove))

(event Custom|Pounce
  (bind _capsulecomponent (Variables|Default|GetCapsuleComponent))
  (bind _returnvalue (Math|Vector|GetForwardVector _capsulecomponent))
  (bind _returnvalue_2 (* _returnvalue 3600))
  (bind _asaic_default_aic (Utilities|Casting|CastToAIC_DefaultAIC (Components|GetOwner)))
  (Variables|/Game/Blueprints/Character/Enemy/AIC_DefaultAIC.AIC_DefaultAIC_C|SetbCanMove _asaic_default_aic false)
  (Variables|/Game/Blueprints/Character/Enemy/AIC_DefaultAIC.AIC_DefaultAIC_C|Setcharging _asaic_default_aic true)
  (Utilities|FlowControl|Delay 1.0)
  (Character|LaunchCharacter (Math|Vector|MakeVector (.x _returnvalue_2) (.y _returnvalue_2) 1e+02) false false)
  (CallFunction|EndSpecialMove))

(event Custom|Leap
  (bind _capsulecomponent (Variables|Default|GetCapsuleComponent))
  (bind _returnvalue (Math|Vector|GetForwardVector _capsulecomponent))
  (bind _returnvalue_2 (* _returnvalue 1000))
  (bind _asaic_default_aic (Utilities|Casting|CastToAIC_DefaultAIC (Components|GetOwner)))
  (Variables|/Game/Blueprints/Character/Enemy/AIC_DefaultAIC.AIC_DefaultAIC_C|SetbCanMove _asaic_default_aic false)
  (Variables|/Game/Blueprints/Character/Enemy/AIC_DefaultAIC.AIC_DefaultAIC_C|Setcharging _asaic_default_aic true)
  (Character|LaunchCharacter (Math|Vector|MakeVector (.x _returnvalue_2) (.y _returnvalue_2) 5e+02) false false)
  (CallFunction|EndSpecialMove))

(event Custom|EndSpecialMove
  (bind _asaic_default_aic (Utilities|Casting|CastToAIC_DefaultAIC (Components|GetOwner)))
  (Variables|/Game/Blueprints/Character/Enemy/AIC_DefaultAIC.AIC_DefaultAIC_C|SetbCanMove _asaic_default_aic true)
  (Variables|/Game/Blueprints/Character/Enemy/AIC_DefaultAIC.AIC_DefaultAIC_C|Setcharging _asaic_default_aic false)
  (Utilities|FlowControl|Delay 6.0)
  (Variables|Default|SetSpcialMoveActive false))

(event EventBeginPlay
  (Variables|Default|SetDefaultStats (Utilities|Struct|MakeS_EnemyStats 5e+01 6e+02 2e+01 1e+02 0.25 1e+02 1.0))
  (|CallParentFunction))

(event EventTick
  (params (DeltaSeconds :type Float%20%28single-precision%29))
  (if (not (Variables|Default|GetSpcialMoveActive))
    (CallFunction|SpecialMove)))

(event EventTryAttack
  (if (Variables|Default|GetbCanAttack)
    (Variables|Default|SetbCanAttack false)
    (Rendering|Material|SetMaterial (Variables|Default|GetTEMP_STATIC_EnemyMesh) 0 "/Game/Assets/Materials/Character/Enemy/M_enemyAttack.M_enemyAttack")
    (Utilities|Time|SetTimerbyEvent (delegate Custom|OnEndAttack) (Variables|Default|GetAttackLandTime))
    (Utilities|Time|SetTimerbyEvent (delegate Custom|ResetAttackGate) (Variables|Default|GetTimeBetweenAttacks))))

(fn ConstructionScript
  (|CallParentFunction))

(fn SpecialMove
  (bind _capsulecomponent (Variables|Default|GetCapsuleComponent))
  (bind _returnvalue (Transformation|GetWorldLocation _capsulecomponent))
  (bind _outhits (Class|KismetSystemLibrary|BoxTraceMultibyProfile _returnvalue (+ _returnvalue (Math|Vector|ClampVectorSize (* (- _returnvalue (Transformation|GetActorLocation (Game|GetPlayerCharacter 0))) -1.0) 0.0 4.5e+02)) "0, 0, 0" "0, 0, 0" "None" false 0 "ForOneFrame" true))
  (if (== (.HitActor (Collision|BreakHitResult (Utilities|Array|Get(acopy) _outhits (Utilities|Array|LastIndex _outhits)))) (Game|GetPlayerCharacter 0))
    (Variables|Default|SetSpcialMoveActive true)
    (switch int (Math|Random|RandomIntegerinRange 0 2)
      (:0
        (CallFunction|Pounce))
      (:1
        (CallFunction|Leap))
      (:2
        (CallFunction|Hunting)))))