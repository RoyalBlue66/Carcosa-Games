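; BP_EnemyKing is a support enemy that buffs other enemies near it through a BuffZone overlap component.
; BP_EnemyBase actors entering the zone get BuffActivate, and those leaving get BuffDeactivate.
; On BeginPlay it deactivates the zone, sets its DefaultStats, runs the parent setup, then reactivates the zone after a short delay.
; Its TryAttack event is empty, with no attack logic of its own.
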(event OnComponentBeginOverlap(BuffZone)
  (params (OverlappedComponent :type Primitive%20Component%20Object%20Reference) (OtherActor :type Actor%20Object%20Reference) (OtherComp :type Primitive%20Component%20Object%20Reference) (OtherBodyIndex :type Integer) (bFromSweep :type Boolean) (SweepResult :type Hit%20Result%20Structure%20%28by%20ref%29))
  ;[1 1 1] Call Enemy Buff Effect
  (bind _asbp_enemy_base (Utilities|Casting|CastToBP_EnemyBase OtherActor))
  (Default|BuffActivate _asbp_enemy_base))

(event OnComponentEndOverlap(BuffZone)
  (params (OverlappedComponent :type Primitive%20Component%20Object%20Reference) (OtherActor :type Actor%20Object%20Reference) (OtherComp :type Primitive%20Component%20Object%20Reference) (OtherBodyIndex :type Integer))
  ;[1 1 1] Call Enemy Return To Normal Effect
  (bind _asbp_enemy_base (Utilities|Casting|CastToBP_EnemyBase OtherActor))
  (Default|BuffDeactivate _asbp_enemy_base))

(event EventTryAttack)

(event EventBeginPlay
  (Components|Activation|Deactivate (Variables|Default|GetBuffZone))
  (Variables|Default|SetDefaultStats (Utilities|Struct|MakeS_EnemyStats 1e+02 3e+02 0.0 6e+02 0.5 1e+02 1.5))
  (|CallParentFunction)
  (Utilities|FlowControl|Delay 0.2)
  (Components|Activation|Activate (Variables|Default|GetBuffZone) false))

(fn ConstructionScript)