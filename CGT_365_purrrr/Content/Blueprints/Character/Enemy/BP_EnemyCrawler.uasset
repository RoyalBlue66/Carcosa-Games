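; BP_EnemyCrawler is an enemy character whose attack slows down the player.
; BeginPlay fills in its DefaultStats before running the parent's BeginPlay.
; TryAttack calls SlowDown on the player character, gated by a CanAttack flag that a timer resets after TimeBetweenAttacks.
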(event Custom|ResetAttack
  ;[1 1 1] Slow Down Player Character On Hit
  (Variables|Default|SetbCanAttack true))

(event EventTryAttack
  ;[1 1 1] Slow Down Player Character On Hit
  (if (Variables|Default|GetbCanAttack)
    (Variables|Default|SetbCanAttack false)
    (bind _asbp_third_person_character (Utilities|Casting|CastToBP_ThirdPersonCharacter (Game|GetPlayerCharacter 0)))
    (Default|SlowDown _asbp_third_person_character)
    (Utilities|Time|SetTimerbyEvent (delegate Custom|ResetAttack) (Variables|Default|GetTimeBetweenAttacks))))

(event EventBeginPlay
  (Variables|Default|SetDefaultStats (Utilities|Struct|MakeS_EnemyStats 1e+02 2e+02 0.0 125.0 0.5 1e+02 1.5))
  (|CallParentFunction))

(fn ConstructionScript)