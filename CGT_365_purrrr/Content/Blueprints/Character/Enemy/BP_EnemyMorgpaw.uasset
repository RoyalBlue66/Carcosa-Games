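; BP_EnemyMorgpaw is an enemy character Blueprint that handles the Morgpaw's damage attacks on the player.
; TryAttack is gated by CanAttack and applies EnemyStats damage to the player without a range check.
; A timer then re-enables attacking after TimeBetweenAttack, which shortens when HasBuff is set.
; A separate IsPlayerHit function, not called here, applies the same damage if HitBox overlaps the player's capsule.
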(event Custom|ResetAttack
  (Variables|Default|SetbCanAttack true))

(event EventBeginPlay)

(event Collision|EventActorBeginOverlap
  (params (OtherActor :type Actor%20Object%20Reference)))

(event EventTick
  (params (DeltaSeconds :type Float%20%28single-precision%29)))

(event EventTryAttack
  (bind _enemystats (Variables|Default|GetEnemyStats))
  (bind (_attackdamage _worthscore _timebetweenattack) (Utilities|Struct|BreakS_EnemyStats _enemystats))
  (if (Variables|Default|GetbCanAttack)
    (Variables|Default|SetbCanAttack false)
    (bind _asbp_third_person_character (Utilities|Casting|CastToBP_ThirdPersonCharacter (Game|GetPlayerCharacter 0)))
    (Game|Damage|ApplyDamage _asbp_third_person_character _attackdamage 0 0)
    (Utilities|Time|SetTimerbyEvent (delegate Custom|ResetAttack) (/ _timebetweenattack (+ 1.0 (* (Variables|Default|GetHasBuff) 0.3))))))

(fn ConstructionScript)

(fn IsPlayerHit
  (bind _returnvalue (Game|GetPlayerCharacter 0))
  (bind _asbp_third_person_character (Utilities|Casting|CastToBP_ThirdPersonCharacter _returnvalue))
  (if (Class|PrimitiveComponent|IsOverlappingComponent (Variables|Default|GetHitBox) (Variables|/Script/Engine.Character|GetCapsuleComponent _asbp_third_person_character))
    (Game|Damage|ApplyDamage _asbp_third_person_character (.AttackDamage (Utilities|Struct|BreakS_EnemyStats (Variables|Default|GetEnemyStats))) 0 0)))