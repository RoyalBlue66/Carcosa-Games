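; BP_EnemyTitan is an enemy character variant that damages the player and periodically knocks them away.
; BeginPlay sets its DefaultStats before calling the parent, then starts a looping timer that prints walk speed.
; TryAttack applies CurrentDamage to the player, with a timer-reset flag as cooldown.
; When knockback is ready, the attack also launches the player along the Titan's forward vector, then recharges on a separate, fixed timer.
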(event Custom|RefreshKnockback
  (Variables|Default|SetKnockback true))

(event Custom|ResetAttack
  (Variables|Default|SetbCanAttack true))

(event Custom|CustomEvent
  (Development|PrintString (Utilities|String|ToString(Float) (Variables|/Script/Engine.CharacterMovementComponent|GetMaxWalkSpeed (Variables|Character|GetCharacterMovement)))))

(event EventTryAttack
  (if (Variables|Default|GetbCanAttack)
    (Variables|Default|SetbCanAttack false)
    (bind _asbp_third_person_character (Utilities|Casting|CastToBP_ThirdPersonCharacter (Game|GetPlayerCharacter 0)))
    (Game|Damage|ApplyDamage _asbp_third_person_character (Variables|Default|GetCurrentDamage) 0 0)
    (Utilities|Time|SetTimerbyEvent (delegate Custom|ResetAttack) (Variables|Default|GetTimeBetweenAttacks))
    (if (Variables|Default|GetKnockback)
      (Variables|Default|SetKnockback false)
      (Character|LaunchCharacter (Game|GetPlayerCharacter 0) (* (Transformation|GetActorForwardVector) "1300.000000,1300.000000,1300.000000") false false)
      (Utilities|Time|SetTimerbyEvent (delegate Custom|RefreshKnockback) 2e+01))))

(event EventBeginPlay
  (Variables|Default|SetDefaultStats (Utilities|Struct|MakeS_EnemyStats 5e+02 2e+02 2e+01 3e+02 0.5 1e+02 1.5))
  (|CallParentFunction)
  (Utilities|Time|SetTimerbyEvent (delegate Custom|CustomEvent) 1.0 true))

(fn ConstructionScript)