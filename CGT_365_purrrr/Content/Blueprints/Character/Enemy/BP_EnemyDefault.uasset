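; BP_EnemyDefault is an enemy that performs timed, telegraphed attacks against the third-person player character.
; TryAttack, gated by a cooldown, swaps the placeholder mesh to an attack material and starts timers for hit landing and cooldown reset.
; DamageArea overlaps set and clear the target reference.
; When the hit timer fires, the material reverts and a still-valid target takes the current damage.
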(event OnComponentBeginOverlap(DamageArea)
  (params (OverlappedComponent :type Primitive%20Component%20Object%20Reference) (OtherActor :type Actor%20Object%20Reference) (OtherComp :type Primitive%20Component%20Object%20Reference) (OtherBodyIndex :type Integer) (bFromSweep :type Boolean) (SweepResult :type Hit%20Result%20Structure%20%28by%20ref%29))
  (bind _asbp_third_person_character (Utilities|Casting|CastToBP_ThirdPersonCharacter OtherActor))
  (Variables|Default|SetAttackTargetRef _asbp_third_person_character))

(event OnComponentEndOverlap(DamageArea)
  (params (OverlappedComponent :type Primitive%20Component%20Object%20Reference) (OtherActor :type Actor%20Object%20Reference) (OtherComp :type Primitive%20Component%20Object%20Reference) (OtherBodyIndex :type Integer))
  (Utilities|Casting|CastToBP_ThirdPersonCharacter OtherActor)
  (Variables|Default|SetAttackTargetRef 0))

(event Custom|OnEndAttack
  (bind _attacktargetref (Variables|Default|GetAttackTargetRef))
  (Rendering|Material|SetMaterial (Variables|Default|GetTEMP_STATIC_EnemyMesh) 0 "/Game/Assets/Materials/Character/Enemy/M_enemy01.M_enemy01")
  (Utilities|IsValid _attacktargetref
    (:Is%20Valid
      (bind _asbp_third_person_character (Utilities|Casting|CastToBP_ThirdPersonCharacter _attacktargetref))
      (Default|OnTakeDamage _asbp_third_person_character (Variables|Default|GetCurrentDamage))
      (Development|PrintString "Hit"))))

(event Custom|ResetAttackGate
  (Variables|Default|SetbCanAttack true))

(event EventBeginPlay
  (|CallParentFunction) ; This node is disabled and will not be called.\nDrag off pins to build functionality.
)

(event EventTryAttack
  (if (Variables|Default|GetbCanAttack)
    (Variables|Default|SetbCanAttack false)
    (Rendering|Material|SetMaterial (Variables|Default|GetTEMP_STATIC_EnemyMesh) 0 "/Game/Assets/Materials/Character/Enemy/M_enemyAttack.M_enemyAttack")
    (Utilities|Time|SetTimerbyEvent (delegate Custom|OnEndAttack) (Variables|Default|GetAttackLandTime))
    (Utilities|Time|SetTimerbyEvent (delegate Custom|ResetAttackGate) (Variables|Default|GetTimeBetweenAttacks))))

(fn ConstructionScript
  (|CallParentFunction))