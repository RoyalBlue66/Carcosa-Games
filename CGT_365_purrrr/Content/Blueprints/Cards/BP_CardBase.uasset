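; BP_CardBase is a spinning card pickup that gives the player a random card when collected.
; Tick adds a fixed yaw step each frame, independent of delta time.
; When the BP_ThirdPersonCharacter capsule overlaps CollectBox, it picks one of the first three DT_Cards rows at random.
; It passes that row's name, uses and texture to the HUD's card hand, then destroys itself.
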(event OnComponentBeginOverlap(CollectBox)
  (params (OverlappedComponent :type Primitive%20Component%20Object%20Reference) (OtherActor :type Actor%20Object%20Reference) (OtherComp :type Primitive%20Component%20Object%20Reference) (OtherBodyIndex :type Integer) (bFromSweep :type Boolean) (SweepResult :type Hit%20Result%20Structure%20%28by%20ref%29))
  (bind _asbp_third_person_character (Utilities|Casting|CastToBP_ThirdPersonCharacter OtherActor))
  (if (== (Variables|/Script/Engine.Character|GetCapsuleComponent _asbp_third_person_character) OtherComp)
    (bind _outrownames (DataTable|GetDataTableRowNames "/Game/Blueprints/Data/Cards/DT_Cards.DT_Cards"))
    (bind _returnvalue (Utilities|GetDataTableRow "/Game/Blueprints/Data/Cards/DT_Cards.DT_Cards" (Utilities|Array|Get(acopy) _outrownames (Math|Random|RandomIntegerinRange 0 2)))
      (:then
        (Class|IFCardControl|AddCard(Message) (Variables|/Game/Blueprints/UI/GUI_HUD/HUD_Container.HUD_Container_C|GetCRD_Hand (Variables|/Game/Blueprints/Character/Player/BP_ThirdPersonCharacter.BP_ThirdPersonCharacter_C|GetHUD%20Container _asbp_third_person_character)) true (.name _returnvalue) (.uses _returnvalue) (.texture _returnvalue))
        (Actor|DestroyActor)))))

(event EventBeginPlay)

(event Collision|EventActorBeginOverlap
  (params (OtherActor :type Actor%20Object%20Reference)))

(event EventTick
  (params (DeltaSeconds :type Float%20%28single-precision%29))
  (bind _returnvalue (Transformation|GetActorRotation))
  (Transformation|SetActorRotation (Math|Rotator|MakeRotator (.roll _returnvalue) (.pitch _returnvalue) (+ (.yaw _returnvalue) 0.6))))

(fn ConstructionScript)