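; BP_VaseBomb is a proximity bomb that starts a short fuse when an enemy comes within range.
; An overlap on its explosion sphere counts only when it hits the capsule of a BP_EnemyBase, which sets a timer.
; When the timer fires, it applies full radial damage around its cube mesh, ignoring the player character, then destroys itself.
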(event OnComponentBeginOverlap(ExplosionSphere)
  (params (OverlappedComponent :type Primitive%20Component%20Object%20Reference) (OtherActor :type Actor%20Object%20Reference) (OtherComp :type Primitive%20Component%20Object%20Reference) (OtherBodyIndex :type Integer) (bFromSweep :type Boolean) (SweepResult :type Hit%20Result%20Structure%20%28by%20ref%29))
  ;[1 1 1] Set Fuse When Enemy Enters Range
  (bind _asbp_enemy_base (Utilities|Casting|CastToBP_EnemyBase OtherActor))
  (if (== (Variables|/Script/Engine.Character|GetCapsuleComponent _asbp_enemy_base) OtherComp)
    (Utilities|Time|SetTimerbyEvent (delegate Custom|Boom) 1.0)))

(event Custom|Boom
  ;[1 1 1] Damage All Enemies In The Area
  (bind _asbp_third_person_character (Utilities|Casting|CastToBP_ThirdPersonCharacter (Game|GetPlayerCharacter 0)))
  (Game|Damage|ApplyRadialDamage 5e+01 (Transformation|GetWorldLocation (Variables|Default|GetCube)) 2e+02 0 (Utilities|Array|MakeArray _asbp_third_person_character) 0 0 true "ECC_Visibility")
  (Actor|DestroyActor))

(event EventBeginPlay)

(event Collision|EventActorBeginOverlap
  (params (OtherActor :type Actor%20Object%20Reference)))

(event EventTick
  (params (DeltaSeconds :type Float%20%28single-precision%29)))

(fn ConstructionScript)