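; Game instance that manages the persistent high score table through an SG_HighScores save game.
; On Init, LoadScores caches the save from its slot, creating and saving a new one if none exists.
; SubmitScores inserts a record ahead of the first lower score or at the end, removes overflow at the MaxRecords index, then writes back through SaveScores.
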(event EventInit
  (CallFunction|LoadScores))

(fn LoadScores
  (if (Utilities|IsValid (Variables|Default|GetCached))
    (return (Variables|Default|GetCached))
    (else
      (bind _returnvalue (SaveGame|DoesSaveGameExist (Variables|Default|GetSlotName)))
      (if _returnvalue
        (bind _returnvalue_2 (SaveGame|LoadGamefromSlot (Variables|Default|GetSlotName)))
        (bind _assg_high_scores (Utilities|Casting|CastToSG_HighScores _returnvalue_2))
        (bind _output_get (Variables|Default|SetCached _assg_high_scores))
        (return _output_get)
        (else
          (bind _returnvalue_3 (SaveGame|CreateSaveGameObject "/Game/Blueprints/GameState/SG_HighScores.SG_HighScores_C"))
          (bind _output_get_2 (Variables|Default|SetCached _returnvalue_3))
          (SaveGame|SaveGametoSlot _output_get_2 (Variables|Default|GetSlotName))
          (return _output_get_2))))))

(fn SaveScores
  (params (Scores :type SG%20High%20Scores%20Object%20Reference))
  (bind _output_get (Variables|Default|SetCached Scores))
  (SaveGame|SaveGametoSlot _output_get (Variables|Default|GetSlotName)))

(fn SubmitScores
  (params (PlayerName :type String) (Score :type Integer))
  (bind _return (CallFunction|LoadScores))
  (bind _output_get (LocalVariables|SetLoadedSave _return))
  (bind _output_get_2 (LocalVariables|SetHighscoreArray (Variables|/Game/Blueprints/GameState/SG_HighScores.SG_HighScores_C|GetHighScores _output_get)))
  (LocalVariables|SetNewRecord (Utilities|Struct|MakeS_ScoreRecord PlayerName Score))
  (if (== (Utilities|Array|Length _output_get_2) 0)
    (Utilities|Array|Insert (LocalVariables|GetHighscoreArray) (LocalVariables|GetNewRecord))
    (else
      (bind (_array_element _array_index) (Utilities|Array|ForEachLoopwithBreak (LocalVariables|GetHighscoreArray) :!label _label)
        (:LoopBody
          (Math|Integer|CompareInt (.Score (Utilities|Struct|BreakS_ScoreRecord (LocalVariables|GetNewRecord))) (.Score (Utilities|Struct|BreakS_ScoreRecord _array_element))
            (:>
              (LocalVariables|SetInsertIndex _array_index)
              (goto _label Break))))
        (:Completed
          (if (== (LocalVariables|GetInsertIndex) -1)
            (LocalVariables|SetInsertIndex (Utilities|Array|Length (LocalVariables|GetHighscoreArray))))
          (Utilities|Array|Insert (LocalVariables|GetHighscoreArray) (LocalVariables|GetNewRecord) (LocalVariables|GetInsertIndex))))))
  (if (> (Utilities|Array|Length (LocalVariables|GetHighscoreArray)) (Variables|/Game/Blueprints/GameState/SG_HighScores.SG_HighScores_C|GetMaxRecords (LocalVariables|GetLoadedSave)))
    (Utilities|Array|RemoveIndex (LocalVariables|GetHighscoreArray) (Variables|/Game/Blueprints/GameState/SG_HighScores.SG_HighScores_C|GetMaxRecords (LocalVariables|GetLoadedSave))))
  (Variables|/Game/Blueprints/GameState/SG_HighScores.SG_HighScores_C|SetHighScores (LocalVariables|GetLoadedSave) (LocalVariables|GetHighscoreArray))
  (CallFunction|SaveScores (LocalVariables|GetLoadedSave)))